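; BP_PersonajeSamurai is the 2D flipbook samurai player character, driven by Enhanced Input through IMC_Samurai, which it registers on BeginPlay.
; Movement runs along world X, and the sign of acceleration snaps control yaw to 0 or 180 to face the travel direction.
; Attack swaps the sprite to FB_Attack with no revert here and also feeds movement input.
; Jump uses the built-in character jump, while the interact action is an empty stub.
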(event `self.ReceiveBeginPlay`
  (bind _asplayer_controller (cast `PlayerController` (`self.GetController`)))
  (message `EnhancedInputSubsystemInterface.AddMappingContext` (pcsubsystem `EnhancedInputLocalPlayerSubsystem` _asplayer_controller) "/Game/2D/Characters/Inputs/Mapping/IMC_Samurai.IMC_Samurai" 0 (struct)))

(event `EnhancedInput|/Game/2D/Characters/Inputs/IA_MovSam`
  (params (ActionValue :type "Float (double-precision)") (ElapsedSeconds :type "Float (double-precision)") (TriggeredSeconds :type "Float (double-precision)") (InputAction :type "InputAction Object Reference" :default "/Game/2D/Characters/Inputs/IA_MovSam.IA_MovSam"))
  (bind _returnvalue (`self.GetController`))
  (bind _returnvalue_x (`KismetMathLibrary.BreakVector` (`CharacterMovementComponent.GetCurrentAcceleration` (`self.CharacterMovement`))))
  (:`Triggered`
    (`self.AddMovementInput` (1.0 0.0 0.0) ActionValue)
    (`/Engine/EditorBlueprintResources/StandardMacros.CompareFloat` _returnvalue_x
      (:`>`
        (`Controller.SetControlRotation` _returnvalue (`KismetMathLibrary.MakeRotator` 0.0)))
      (:`<`
        (`Controller.SetControlRotation` _returnvalue (`KismetMathLibrary.MakeRotator` 0.0 0.0 180.0))))))

(event `EnhancedInput|/Game/2D/Characters/Inputs/IA_AttackSam`
  (params (ActionValue :type "Float (double-precision)") (ElapsedSeconds :type "Float (double-precision)") (TriggeredSeconds :type "Float (double-precision)") (InputAction :type "InputAction Object Reference" :default "/Game/2D/Characters/Inputs/IA_AttackSam.IA_AttackSam"))
  (:`Started`
    (`PaperFlipbookComponent.SetFlipbook` (`self.Sprite`) "/Game/2D/Sprite/Attack/FB_Attack.FB_Attack")
    (`self.AddMovementInput` (1.0 0.0 0.0) ActionValue)))

(event `EnhancedInput|/Game/2D/Characters/Inputs/IA_InteractuarSam`
  (params (ActionValue :type "Float (double-precision)") (ElapsedSeconds :type "Float (double-precision)") (TriggeredSeconds :type "Float (double-precision)") (InputAction :type "InputAction Object Reference" :default "/Game/2D/Characters/Inputs/IA_InteractuarSam.IA_InteractuarSam")))

(event `EnhancedInput|/Game/2D/Characters/Inputs/IA_JumpSam`
  (params (ActionValue :type "Float (double-precision)") (ElapsedSeconds :type "Float (double-precision)") (TriggeredSeconds :type "Float (double-precision)") (InputAction :type "InputAction Object Reference" :default "/Game/2D/Characters/Inputs/IA_JumpSam.IA_JumpSam"))
  (:`Started`
    (`self.Jump`)))

(fn `UserConstructionScript`)