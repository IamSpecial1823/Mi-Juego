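; BP_Personaje is a player-controlled character Blueprint with basic movement, turning and jumping through Enhanced Input.
; On BeginPlay it adds the IMC_PersonajeInput mapping context to the local player's subsystem, provided its controller is a PlayerController.
; IA_Mirar drives controller yaw only, IA_Movimiento moves the character along its forward vector scaled by the input value, and IA_Jump calls Jump whenever triggered.
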(event `self.ReceiveBeginPlay`
  (bind _asplayer_controller (cast `PlayerController` (`self.GetController`)))
  (`EnhancedInputSubsystemInterface.AddMappingContext` (pcsubsystem `EnhancedInputLocalPlayerSubsystem` _asplayer_controller) "/Game/Blueprints/ClaseHerencia/Inputs/MappingContext/IMC_PersonajeInput.IMC_PersonajeInput" 0 (struct)))

(event `EnhancedInput|/Game/Blueprints/ClaseHerencia/Inputs/InputAction/IA_Mirar`
  (params (ActionValue :type "Float (double-precision)") (ElapsedSeconds :type "Float (double-precision)") (TriggeredSeconds :type "Float (double-precision)") (InputAction :type "InputAction Object Reference" :default "/Game/Blueprints/ClaseHerencia/Inputs/InputAction/IA_Mirar.IA_Mirar"))
  (:`Triggered`
    (`self.AddControllerYawInput` ActionValue)))

(event `EnhancedInput|/Game/Blueprints/ClaseHerencia/Inputs/InputAction/IA_Movimiento`
  (params (ActionValue :type "Float (double-precision)") (ElapsedSeconds :type "Float (double-precision)") (TriggeredSeconds :type "Float (double-precision)") (InputAction :type "InputAction Object Reference" :default "/Game/Blueprints/ClaseHerencia/Inputs/InputAction/IA_Movimiento.IA_Movimiento"))
  (:`Triggered`
    (`self.AddMovementInput` (* (`self.GetActorForwardVector`) ActionValue))))

(event `EnhancedInput|/Game/Blueprints/ClaseHerencia/Inputs/InputAction/IA_Jump`
  (params (ActionValue :type "Float (double-precision)") (ElapsedSeconds :type "Float (double-precision)") (TriggeredSeconds :type "Float (double-precision)") (InputAction :type "InputAction Object Reference" :default "/Game/Blueprints/ClaseHerencia/Inputs/InputAction/IA_Jump.IA_Jump"))
  (:`Triggered`
    (`self.Jump`)))

(fn `UserConstructionScript`)